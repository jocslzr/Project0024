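; BP_Climb_Trigger is a demo volume that marks where the ThirdPersonCharacter can climb.
; When the character begins overlapping its Box, it sets the character's Climbing flag to true.
; On end overlap, it clears the flag only if the character's capsule overlaps no other trigger of the same class, so adjacent or overlapping volumes keep climbing active.
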(event OnComponentBeginOverlap(Box)
  (params (OverlappedComponent :type Primitive%20Component%20Object%20Reference) (OtherActor :type Actor%20Object%20Reference) (OtherComp :type Primitive%20Component%20Object%20Reference) (OtherBodyIndex :type Integer) (bFromSweep :type Boolean) (SweepResult :type Hit%20Result%20Structure%20%28by%20ref%29))
  (bind _asthird_person_character (Utilities|Casting|CastToThirdPersonCharacter OtherActor))
  (Variables|/Game/SimpleClimbingAnims/DemoContent/Blueprints/ThirdPersonCharacter.ThirdPersonCharacter_C|SetbClimbing _asthird_person_character true))

(event OnComponentEndOverlap(Box)
  (params (OverlappedComponent :type Primitive%20Component%20Object%20Reference) (OtherActor :type Actor%20Object%20Reference) (OtherComp :type Primitive%20Component%20Object%20Reference) (OtherBodyIndex :type Integer))
  (bind _asthird_person_character (Utilities|Casting|CastToThirdPersonCharacter OtherActor))
  (if (not (Utilities|Array|IsValidIndex (Collision|GetOverlappingActors (Variables|/Script/Engine.Character|GetCapsuleComponent _asthird_person_character) (Utilities|GetClass self) :!class /Script/Engine.PrimitiveComponent)))
    (Variables|/Game/SimpleClimbingAnims/DemoContent/Blueprints/ThirdPersonCharacter.ThirdPersonCharacter_C|SetbClimbing _asthird_person_character false)))

(fn ConstructionScript)