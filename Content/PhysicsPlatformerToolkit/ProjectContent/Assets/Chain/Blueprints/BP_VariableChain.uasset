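; Physics chain actor that builds a variable number of links along the line from BeginLocation to EndLocation in the Construction Script.
; It places the existing first and last links, fills between them with simulated copies of FirstLink, and rotates every other link.
; Physics constraints join neighboring links, copying limits and angular drive settings from LinkAttachment, a template component destroyed on BeginPlay.
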(event EventBeginPlay
  (Components|DestroyComponent (Variables|Default|GetLinkAttachment)) ; This component is only used during construction for configuration, \nso there's no need to keep it after we start the game.
)

(fn ConstructionScript
  (CallFunction|ConstructChain))

(fn ConstructChain
  (bind _beginlocation (Variables|BeginOfChain|GetBeginLocation))
  (bind _endlocation (Variables|EndOfChain|GetEndLocation))
  (bind _lastlink (Variables|Default|GetLastLink))
  (bind _distancebetweenlinks (Variables|WholeChainConfig|GetDistanceBetweenLinks))
  (bind _firstlink (Variables|Default|GetFirstLink))
  (bind _returnvalue (- _beginlocation _endlocation))
  (bind _returnvalue_2 (Math|Vector|VectorLength _returnvalue))
  (bind _returnvalue_3 (/ _returnvalue_2 _distancebetweenlinks))
  (bind _returnvalue_4 (Math|Float|Floor _returnvalue_3))
  (bind _returnvalue_5 (- _returnvalue_4 2))
  (LocalVariables|SetChainDirection (Math|Vector|Normalize (- (Variables|EndOfChain|GetEndLocation) (Variables|BeginOfChain|GetBeginLocation)))) ; Direction along which the chain will be created.
  ;[1 1 1] Place first link (which is already created)
  (Transformation|SetRelativeTransform _firstlink (Math|Transform|MakeTransform (+ (* (Variables|WholeChainConfig|GetDistanceBetweenLinks) (LocalVariables|GetChainDirection)) (Variables|BeginOfChain|GetBeginLocation)) (Math|Rotator|MakeRotfromX (LocalVariables|GetChainDirection)) (Variables|WholeChainConfig|GetLinkScale)) false false)
  (Class|PrimitiveComponent|SetPhysMaterialOverride _firstlink (Variables|WholeChainConfig|GetLinkPhysicalMaterial))
  (Class|PrimitiveComponent|SetConstraintMode _firstlink (Variables|WholeChainConfig|GetConstraint%20Mode))
  (Class|PrimitiveComponent|SetMassOverrideinKg _firstlink "None" (Variables|WholeChainConfig|GetLinkMass) true)
  (LocalVariables|SetPreviousLink _firstlink)
  (for _index (range 0 _returnvalue_5) ; Go through the rest of the links
    (if (== _index _returnvalue_5) ; Have we reached the last link?
      ;[1 1 1] Place the last link (which is already created)
      (Transformation|SetWorldTransform _lastlink (Math|Transform|MakeTransform (+ (* (Variables|WholeChainConfig|GetDistanceBetweenLinks) (LocalVariables|GetChainDirection)) (Transformation|GetWorldLocation (LocalVariables|GetPreviousLink))) (Math|Rotator|MakeRotfromX (LocalVariables|GetChainDirection)) (Variables|WholeChainConfig|GetLinkScale)) false false)
      (Class|PrimitiveComponent|SetPhysMaterialOverride _lastlink (Variables|WholeChainConfig|GetLinkPhysicalMaterial))
      (Class|PrimitiveComponent|SetMassOverrideinKg _lastlink "None" (Variables|WholeChainConfig|GetLinkMass) true)
      (Class|PrimitiveComponent|SetConstraintMode _lastlink (Variables|WholeChainConfig|GetConstraint%20Mode))
      (else
        ;[1 1 1] Create other links
        (bind _createdlink (CallFunction|CreateLink (Transformation|GetWorldLocation (LocalVariables|GetPreviousLink)) (LocalVariables|GetChainDirection)))))
    ;[1 1 1] Rotate link if odd index
    (if (not (> (Math|Integer|%(Integer) _index 2) 0)) ; Select odd indexes
      (Transformation|AddLocalRotation (select (== _index _returnvalue_5) (Variables|Default|GetLastLink) _createdlink) "0.000000,0.000000,90.000000" false false) ; Rotate chain link to be perpendicular to the last one
    )
    ;[1 1 1] Create and configure attachement between links
    (bind _returnvalue_6 (AddComponent|AddPhysicsConstraintComponent true (Math|Transform|MakeTransform (+ (Transformation|GetWorldLocation (LocalVariables|GetPreviousLink)) (* (Variables|WholeChainConfig|GetPCLinkOffset) (LocalVariables|GetChainDirection))) (Math|Rotator|MakeRotfromX (LocalVariables|GetChainDirection)) "1.000000,1.000000,1.000000")))
    (CallFunction|ConfigurePC _returnvalue_6 (LocalVariables|GetPreviousLink) (select (== _index _returnvalue_5) (Variables|Default|GetLastLink) _createdlink))
    (LocalVariables|SetPreviousLink (select (== _index _returnvalue_5) (Variables|Default|GetLastLink) _createdlink)) ; Remember the previous link
  ))

(fn ConfigurePC
  (params (PhysicsConstraint :type Physics%20Constraint%20Component%20Object%20Reference) (PreviousLink :type Primitive%20Component%20Object%20Reference) (CurrentLink :type Primitive%20Component%20Object%20Reference))
  (Utilities|FlowControl|Sequence
    (:then_0
      (Transformation|AttachComponentToComponent PhysicsConstraint PreviousLink "None" "KeepWorld" "SnapToTarget" "KeepWorld" false)
      (Class|PhysicsConstraintComponent|SetConstrainedComponents PhysicsConstraint PreviousLink "None" CurrentLink "None")
      (Class|PhysicsConstraintComponent|SetDisableCollision PhysicsConstraint true))
    (:then_1
      (bind _returnvalue (Class|PhysicsConstraintComponent|GetConstraint PhysicsConstraint))
      (bind _returnvalue_2 (Class|PhysicsConstraintComponent|GetConstraint (Variables|Default|GetLinkAttachment)))
      (bind (_xmotion _ymotion _zmotion _limit) (Class|ConstraintInstanceBlueprintLibrary|GetLinearLimits _returnvalue_2))
      (Class|ConstraintInstanceBlueprintLibrary|SetLinearLimits _returnvalue _xmotion _ymotion _zmotion _limit)
      (bind (_swing1motiontype _swing1limitangle _swing2motiontype _swing2limitangle _twistmotiontype _twistlimitangle) (Class|ConstraintInstanceBlueprintLibrary|GetAngularLimits _returnvalue_2))
      (Class|ConstraintInstanceBlueprintLibrary|SetAngularLimits _returnvalue _swing1motiontype _swing1limitangle _swing2motiontype _swing2limitangle _twistmotiontype _twistlimitangle)
      (bind _outdrivemode (Class|ConstraintInstanceBlueprintLibrary|GetAngularDriveMode _returnvalue_2))
      (Class|ConstraintInstanceBlueprintLibrary|SetAngularDriveMode _returnvalue _outdrivemode)
      (bind (_outpositionstrength _outvelocitystrength _outforcelimit) (Class|ConstraintInstanceBlueprintLibrary|GetAngularDriveParams _returnvalue_2))
      (Class|ConstraintInstanceBlueprintLibrary|SetAngularDriveParams _returnvalue _outpositionstrength _outvelocitystrength _outforcelimit)
      (bind _outveltarget (Class|ConstraintInstanceBlueprintLibrary|GetAngularVelocityTarget _returnvalue_2))
      (Class|ConstraintInstanceBlueprintLibrary|SetAngularVelocityTarget _returnvalue _outveltarget)
      (bind _outpostarget (Class|ConstraintInstanceBlueprintLibrary|GetAngularOrientationTarget _returnvalue_2))
      (Class|ConstraintInstanceBlueprintLibrary|SetAngularOrientationTarget _returnvalue _outpostarget))))

(fn CreateLink
  (params (LastLinkWorldLocation :type Vector) (ChainDirection :type Vector))
  ;[1 1 1] Create  Link and copy properties from FirstLink
  (bind _returnvalue (AddComponent|AddStaticMeshComponent true (Math|Transform|MakeTransform (+ (* (Variables|WholeChainConfig|GetDistanceBetweenLinks) ChainDirection) LastLinkWorldLocation) (Math|Rotator|MakeRotfromX ChainDirection) (Variables|WholeChainConfig|GetLinkScale))))
  (Class|PrimitiveComponent|SetConstraintMode _returnvalue (Variables|WholeChainConfig|GetConstraint%20Mode))
  (Components|StaticMesh|SetStaticMesh _returnvalue (Variables|/Script/Engine.StaticMeshComponent|GetStaticMesh (Variables|Default|GetFirstLink)))
  (Class|PrimitiveComponent|SetMassOverrideinKg _returnvalue "None" (Physics|GetMass (Variables|Default|GetFirstLink)) true)
  (Physics|SetSimulatePhysics _returnvalue true)
  (Rendering|Material|SetMaterial _returnvalue 0 (Rendering|Material|GetMaterial (Variables|Default|GetFirstLink) 0))
  (Class|PrimitiveComponent|SetPhysMaterialOverride _returnvalue (Variables|WholeChainConfig|GetLinkPhysicalMaterial))
  (return _returnvalue))