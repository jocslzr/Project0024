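; Enemy rifle projectile Blueprint that relays its collision hits as projectile impacts.
; On BeginPlay, its box collision ignores the instigator, or the owner if no valid instigator exists, while moving.
; Box hits call OnProjectileImpact with the hit actor and result; the impact response is not defined in this graph.
; The remaining functions, which resemble an enemy AI interface, are stubs returning default values.
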(event OnComponentHit(BoxCollision)
  (params (HitComponent :type Primitive%20Component%20Object%20Reference) (OtherActor :type Actor%20Object%20Reference) (OtherComp :type Primitive%20Component%20Object%20Reference) (NormalImpulse :type Vector :default "0, 0, 0") (Hit :type Hit%20Result%20Structure%20%28by%20ref%29))
  (Default|CallOnProjectileImpact OtherActor Hit))

(event EventBeginPlay
  (bind _returnvalue (Game|GetInstigator))
  (|CallParentFunction)
  (Collision|IgnoreActorwhenMoving (Variables|Default|GetBoxCollision) (select (Utilities|IsValid _returnvalue) _returnvalue (Components|GetOwner)) true))

(fn ConstructionScript
  (|CallParentFunction))

(fn AttackStart
  (params (AttackTarget :type Actor%20Object%20Reference) (TokensNeeded :type Integer))
  (return false))

(fn GetExternalShieldGenerator
  (return 0))

(fn GetIdealRange
  (return 0.0 0.0 0.0))

(fn GetKnockDownCount
  (return 0))

(fn GetPatrolRoute
  (return 0))

(fn GetVantagePoints
  (return 0))

(fn GetWithinWindowStatus
  (return true))

(fn HasShield
  (return false))

(fn SetMovementSpeed
  (params (Speed :type E_MovingSpeed%20Enum :default "NewEnumerator0"))
  (return 0.0))