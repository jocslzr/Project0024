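; Ground attack AOE actor that places itself on the surface at its Target before firing.
; On BeginPlay it runs the parent logic, calls MoveToFloor, then Trigger.
; MoveToFloor line-traces from a valid Target, scaling its location's Z by -1000 for the end point rather than subtracting an offset, with debug drawing on.
; On a hit it spawns a land crack emitter and moves the actor there.
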(event Custom|MoveToFloor
  (bind _target (Variables|Default|GetTarget)
    (:then
      (bind (_outhit _returnvalue) (Collision|LineTraceByChannel (Transformation|GetActorLocation _target) (* (Transformation|GetActorLocation _target) "1.000000,1.000000,-1000.000000") "TraceTypeQuery1" false (Utilities|Array|MakeArray _target) "ForDuration"))
      (if _returnvalue
        (Effects|SpawnEmitteratLocation "/Game/Stylized_FX4/ParticleSystem/LandCrack/P_LandCrack.P_LandCrack" (.ImpactPoint (Collision|BreakHitResult _outhit)))
        (Transformation|SetActorLocation (.Location (Collision|BreakHitResult _outhit)) false false)))
    (:else)))

(event EventBeginPlay
  (|CallParentFunction)
  (CallFunction|MovetoFloor)
  (CallFunction|Trigger))

(fn ConstructionScript
  (|CallParentFunction))