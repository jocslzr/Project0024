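; Blueprint function library that looks up input prompt icon textures for PC keys, PlayStation buttons and Xbox buttons.
; Each platform has its own function, which picks a Light or Dark data table from the Theme input.
; The key's display name, passed through an underscore string replace, becomes the row name, and the function returns that row's Icon.
; Missing rows get no special handling.
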(fn GetPCKeyTexture
  (params (Key :type Key%20Structure :default "A") (Theme :type InputIconTheme%20Enum :default "NewEnumerator0"))
  (bind _returnvalue (Utilities|GetDataTableRow (Utilities|Select :Index Theme :NewEnumerator0 "/Game/InputKeysIconPack/DataTables/_SearchTables/DT_PC_SearchTable.DT_PC_SearchTable" :NewEnumerator1 "/Game/InputKeysIconPack/DataTables/_SearchTables/DT_PC-Dark_SearchTable.DT_PC-Dark_SearchTable") (Utilities|String|StringToName (Utilities|String|Replace (Utilities|String|ToString(Text) (Class|KismetInputLibrary|KeyGetDisplayName Key)) " " "_")))
    (:then
      _)
    (:RowNotFound
      _))
  (return (Utilities|Struct|BreakFInputIconRow _returnvalue)))

(fn GetPSButtonTexture
  (params (Button :type Key%20Structure :default "A") (Theme :type InputIconTheme%20Enum :default "NewEnumerator0"))
  (bind _returnvalue (Utilities|GetDataTableRow (Utilities|Select :Index Theme :NewEnumerator0 "/Game/InputKeysIconPack/DataTables/_SearchTables/DT_PS_SearchTable.DT_PS_SearchTable" :NewEnumerator1 "/Game/InputKeysIconPack/DataTables/_SearchTables/DT_PS-Dark_SearchTable.DT_PS-Dark_SearchTable") (Utilities|String|StringToName (Utilities|String|Replace (Utilities|String|ToString(Text) (Class|KismetInputLibrary|KeyGetDisplayName Button)) " " "_")))
    (:then
      _)
    (:RowNotFound
      _))
  (return (Utilities|Struct|BreakFInputIconRow _returnvalue)))

(fn GetXBButtonTexture
  (params (Button :type Key%20Structure :default "A") (Theme :type InputIconTheme%20Enum :default "NewEnumerator0"))
  (bind _returnvalue (Utilities|GetDataTableRow (Utilities|Select :Index Theme :NewEnumerator0 "/Game/InputKeysIconPack/DataTables/_SearchTables/DT_XB_SearchTable.DT_XB_SearchTable" :NewEnumerator1 "/Game/InputKeysIconPack/DataTables/_SearchTables/DT_XB-Dark_SearchTable.DT_XB-Dark_SearchTable") (Utilities|String|StringToName (Utilities|String|Replace (Utilities|String|ToString(Text) (Class|KismetInputLibrary|KeyGetDisplayName Button)) " " "_")))
    (:then
      _)
    (:RowNotFound
      _))
  (return (Utilities|Struct|BreakFInputIconRow _returnvalue)))