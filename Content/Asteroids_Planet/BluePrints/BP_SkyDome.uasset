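; BP_SkyDome is a sky dome actor that sets up a starry sky material and a matching directional sun light.
; The construction script creates a dynamic material on the sky mesh and feeds it sun, star and sky parameters, taking light direction from the actor's rotation.
; It sets the light's intensity and color, using a separate color variable from the material's tinted sun color.
; A repainting switch selects three repaint colors or one base sky color.
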(fn ConstructionScript
  (bind _directionallight (Variables|Components|GetDirectionalLight))
  (bind _repainting_sky (Variables|Default|GetRepainting%20Sky))
  ;[1 1 1] Create Dynamic Material
  (bind _returnvalue (Rendering|Material|CreateDynamicMaterialInstance (Variables|BP_Skydome|GetSky%20Sphere%20mesh) 0 (Variables|Components|GetSky%20Dome) :!class /Script/Engine.PrimitiveComponent))
  (Variables|Default|SetSky%20material _returnvalue)
  ;[1 1 1] The rotation of the sun,  Sun Intencity
  (Transformation|AddLocalRotation _directionallight "0, 0, 0" false false)
  (Rendering|Components|Light|SetIntensity _directionallight (Variables|Default|GetSun%20Intencity))
  (Rendering|Material|SetVectorParameterValue (Variables|Default|GetSky%20material) "Light direction" (Math|Conversions|ToLinearColor(Vector) (Math|Rotator|GetRotationXVector (Transformation|GetActorRotation))) :!class /Script/Engine.MaterialInstanceDynamic)
  ;[1 1 1] Sun color
  (Rendering|Components|Light|SetLightColor _directionallight (Variables|Default|GetSun%20Color%202) true)
  (Rendering|Material|SetVectorParameterValue (Variables|Default|GetSky%20material) "Sun color" (* (Variables|Default|GetSun%20Color) (Math|Color|Lerp(LinearColor) "(R=0.337500,G=0.337500,B=0.337500,A=1.000000)" "(R=0.954000,G=0.901000,B=0.744120,A=1.000000)" (Math|Float|Clamp(Float) 0.2))) :!class /Script/Engine.MaterialInstanceDynamic)
  ;[1 1 1] Sun brightness
  (Rendering|Material|SetScalarParameterValue (Variables|Default|GetSky%20material) "Sun brightness" (Variables|Default|GetSun%20brightness) :!class /Script/Engine.MaterialInstanceDynamic)
  ;[1 1 1] Stars brightness
  (Rendering|Material|SetScalarParameterValue (Variables|Default|GetSky%20material) "Stars Brightness" (Variables|Default|GetStars%20brightness) :!class /Script/Engine.MaterialInstanceDynamic)
  ;[1 1 1] Sun Radius
  (Rendering|Material|SetScalarParameterValue (Variables|Default|GetSky%20material) "Sun Radius" (Variables|Default|GetSun%20Radius) :!class /Script/Engine.MaterialInstanceDynamic)
  ;[1 1 1] Sky Intensity
  (Rendering|Material|SetScalarParameterValue (Variables|Default|GetSky%20material) "Sky Intensity" (Variables|Default|GetSky%20Intensity) :!class /Script/Engine.MaterialInstanceDynamic)
  ;[1 1 1] Switching to the repainting of the sky
  (Rendering|Material|SetScalarParameterValue (Variables|Default|GetSky%20material) "Repainting Sky" (Math|Conversions|ToFloat(Boolean) _repainting_sky) :!class /Script/Engine.MaterialInstanceDynamic)
  (if _repainting_sky
    ;[1 1 1] repainting of the sky
    (Rendering|Material|SetVectorParameterValue (Variables|Default|GetSky%20material) "Repainting 1" (Variables|Default|GetRepainting%201) :!class /Script/Engine.MaterialInstanceDynamic)
    (Rendering|Material|SetVectorParameterValue (Variables|Default|GetSky%20material) "Repainting 2" (Variables|Default|GetRepainting%202) :!class /Script/Engine.MaterialInstanceDynamic)
    (Rendering|Material|SetVectorParameterValue (Variables|Default|GetSky%20material) "Repainting 3" (Variables|Default|GetRepainting%203) :!class /Script/Engine.MaterialInstanceDynamic)
    (else
      ;[1 1 1] Sky Base Color
      (Rendering|Material|SetVectorParameterValue (Variables|Default|GetSky%20material) "Sky Color" (Variables|Default|GetSky%20Color) :!class /Script/Engine.MaterialInstanceDynamic))))