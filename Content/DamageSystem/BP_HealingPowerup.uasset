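; BP_HealingPowerup is a healing pickup that restores health to the player on contact.
; Overlapping its sphere collision casts to BP_Player and checks the player's BPCDamageSystem component, so pickup only happens below max health.
; It then sends HealMessage with its Amount, spawns an orb pickup particle effect and destroys itself after a short delay.
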(event OnComponentBeginOverlap(SphereCollision)
  (params (OverlappedComponent :type Primitive%20Component%20Object%20Reference) (OtherActor :type Actor%20Object%20Reference) (OtherComp :type Primitive%20Component%20Object%20Reference) (OtherBodyIndex :type Integer) (bFromSweep :type Boolean) (SweepResult :type Hit%20Result%20Structure%20%28by%20ref%29))
  (bind _asbp_player (Utilities|Casting|CastToBP_Player OtherActor))
  (if (< (Variables|/Game/DamageSystem/BPC_DamageSystem.BPC_DamageSystem_C|GetHealth (Variables|/Game/ThirdPerson/Blueprints/Player/BP_Player.BP_Player_C|GetBPC_DamageSystem _asbp_player)) (Variables|/Game/DamageSystem/BPC_DamageSystem.BPC_DamageSystem_C|GetMaxHealth (Variables|/Game/ThirdPerson/Blueprints/Player/BP_Player.BP_Player_C|GetBPC_DamageSystem _asbp_player)))
    (Class|BPIDamageable|Heal(Message) _asbp_player (Variables|Default|GetAmount))
    (Effects|SpawnEmitteratLocation "/Game/InfinityBladeEffects/Effects/FX_Archive/P_HealthOrb_Pickup.P_HealthOrb_Pickup" (Transformation|GetActorLocation) "0, 0, 0" "2.000000,2.000000,2.000000")
    (Utilities|FlowControl|Delay 0.2)
    (Actor|DestroyActor)))

(fn ConstructionScript)