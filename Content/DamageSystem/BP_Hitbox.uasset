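; BP_Hitbox is a damage-system hitbox with a visual display that distinguishes strike boxes from hurtboxes.
; SpawnHitbox picks the strike or hurtbox material from the HitboxType enum, applies it to HitboxDisplay, then moves that component to a given world location without sweeping.
; CheckCollision is an empty stub and the construction script does nothing, so no collision or damage logic runs here.
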(event Custom|SpawnHitbox
  (switch Utilities|FlowControl|Switch|Switchon (Variables|Default|GetHitboxType)
    (:NewEnumerator0
      (Rendering|Material|SetMaterial (Variables|Default|GetHitboxDisplay) 0 (Variables|Default|GetStrikeMaterial)))
    (:NewEnumerator1
      (Rendering|Material|SetMaterial (Variables|Default|GetHitboxDisplay) 0 (Variables|Default|GetHurtboxMaterial))))
  (Transformation|SetWorldLocation (Variables|Default|GetHitboxDisplay) (Variables|Default|GetNew%20Location) false false))

(event Custom|CheckCollision)

(fn ConstructionScript)