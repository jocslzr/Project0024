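; BP_Etasphera04_01 assembles the Etasphera04 figure from separate skeletal mesh components for head, body, armor, arms, individual finger joints and legs.
; Its construction script sets Mesh as the master pose component for the listed parts.
; The parts therefore follow that single mesh's pose and animate as one body, without evaluating animation individually.
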(fn ConstructionScript
  (Class|SkinnedMeshComponent|SetMasterPoseComponent (Variables|Default|GetSK_Etasphera04_Arm_ring_01_r) (Variables|Character|GetMesh)))