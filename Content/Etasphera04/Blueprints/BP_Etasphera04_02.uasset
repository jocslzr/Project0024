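; BP_Etasphera04_02 is a modular Etasphera04 Blueprint assembled from separate skeletal mesh parts for arms, hip and thigh armor, body, plasma head and legs.
; Its construction script sets Mesh as the master pose component for each listed part.
; The parts therefore follow one shared pose from Mesh instead of animating independently.
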(fn ConstructionScript
  (Class|SkinnedMeshComponent|SetMasterPoseComponent (Variables|Default|GetSK_Etasphera04_Arm2_r) (Variables|Character|GetMesh)))